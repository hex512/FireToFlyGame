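; Enemy actor that awards score when hit or killed, with health initialized from its HP on BeginPlay.
; Both Hit and Dead play audio and a timeline scale pulse on the cube, then send score through the GameStateHelper interface.
; If that interface exists, death also spawns an explosion, launches the player toward the enemy's position and destroys the actor.
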(event Custom|HitEffect
  (Audio|Components|Audio|Play (Variables|Default|GetAudio) 0.0)
  (bind _scale (Timeline|Timeline_Scale PlayFromStart)
    (:Update
      (Transformation|SetWorldScale3D (Variables|Default|GetCube) (Math|Vector|MakeVector _scale _scale _scale)))))

(event EventBeginPlay
  (Variables|/Script/JoyWay_HEX512.Healt|SetSetupHealt (Variables|Default|GetHealt) (Variables|Default|GetHP)))

(event EventHit
  (params (ShotFromDirection :type Vector :default "0, 0, 0"))
  (CallFunction|HitEffect)
  (if (Utilities|DoesObjectImplementInterface (Game|GetGameState) "/Script/JoyWay_HEX512.GameStateHelper")
    (Class|GameStateHelper|AddScore(Message) (Game|GetGameState) (Variables|ScoreSettings|GetScoreHit))))

(event EventDead
  (bind _returnvalue (Game|GetPlayerCharacter 0))
  (CallFunction|HitEffect)
  (if (Utilities|DoesObjectImplementInterface (Game|GetGameState) "/Script/JoyWay_HEX512.GameStateHelper")
    (Class|GameStateHelper|AddScore(Message) (Game|GetGameState) (Variables|ScoreSettings|GetScoreDead))
    (Effects|SpawnEmitteratLocation "/Game/Resource/GameDesign/MilitaryWeapDark/FX/P_Grenade_Explosion_01.P_Grenade_Explosion_01" (Transformation|GetActorLocation))
    (Character|LaunchCharacter _returnvalue (* (Math|Vector|GetForwardVector (Math|Rotator|FindLookatRotation (Transformation|GetActorLocation _returnvalue) (Transformation|GetActorLocation))) 2e+03) true true)
    (Actor|DestroyActor)))

(fn ConstructionScript)