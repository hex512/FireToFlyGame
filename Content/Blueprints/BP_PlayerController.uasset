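; Player controller that shows a pause menu on the Escape input action.
; Pressing Escape lazily creates and caches the WBP_EscapeMenu widget, adds it at a high Z-order, switches to UI-only input with the cursor shown, and pauses the game.
; The Released event, rather than a second press, removes the menu, restores game-only input, hides the cursor and unpauses.
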(event EventBeginPlay)

(event EventTick
  (params (DeltaSeconds :type Float%20%28single-precision%29)))

(event Input|ActionEvents|InputActionEscape
  (params (Key :type Key%20Structure :default "None"))
  (:Pressed
    (Variables|Default|GetEscape%20Menu
      (:then
        _)
      (:else
        (bind _returnvalue (UserInterface|CreateWidget "/Game/Blueprints/Menu/WBP_EscapeMenu.WBP_EscapeMenu_C"))
        (Variables|Default|SetEscape%20Menu _returnvalue)))
    (UserInterface|Viewport|AddtoViewport (Variables|Default|GetEscape%20Menu) 999)
    (Input|SetInputModeUIOnly self (Variables|Default|GetEscape%20Menu) "DoNotLock")
    (Variables|Default|SetbShowMouseCursor self true)
    (Game|SetGamePaused true))
  (:Released
    (bind _escape_menu (Variables|Default|GetEscape%20Menu)
      (:then
        (Widget|RemovefromParent _escape_menu))
      (:else
        _))
    (Input|SetInputModeGameOnly self)
    (Variables|Default|SetbShowMouseCursor self false)
    (Game|SetGamePaused false)))

(fn ConstructionScript)