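; BP_Weapon is a pickup gun that a JW_Character takes into a free first (right hand) or second (left hand) slot.
; Taking it attaches and owns the weapon, ignores mesh collision and plays a sound.
; Fire plays an animation and line-traces from player 0's camera, spawning an impact effect and applying point damage, throttled by DoOnce and Delay.
; Debug drawing and printing remain, and GetCurrentAmmo is a stub returning zero.
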(event EventFire
  (bind _returnvalue (Game|GetPlayerCameraManager 0))
  (bind _returnvalue_2 (Transformation|GetActorLocation _returnvalue))
  (Utilities|FlowControl|DoOnce false :!label _label
    (:Completed
      (Utilities|FlowControl|Sequence
        (:then_0
          (Components|Animation|PlayAnimation (Variables|Default|GetWeaponMesh) (Variables|Default|GetFireAnimation) false)
          (bind (_outhit _returnvalue_3) (Collision|LineTraceByChannel _returnvalue_2 (+ _returnvalue_2 (* (Transformation|GetActorForwardVector _returnvalue) 5e+04)) "TraceTypeQuery1" false (Actor|GetAllChildActors (Components|GetOwner) true) "ForDuration"))
          (if _returnvalue_3
            (Effects|SpawnEmitteratLocation "/Game/Resource/GameDesign/MilitaryWeapDark/FX/P_Impact_Stone_Large_01.P_Impact_Stone_Large_01" (.ImpactPoint (Collision|BreakHitResult _outhit)))
            (Utilities|IsValid (.HitActor (Collision|BreakHitResult _outhit))
              (:Is%20Valid
                (Game|Damage|ApplyPointDamage (.HitActor (Collision|BreakHitResult _outhit)) (Variables|Default|GetBase%20Damage) (.ImpactNormal (Collision|BreakHitResult _outhit)) _outhit (Pawn|GetController (Variables|Default|GetAs%20JW%20Character)) self)
                (Development|PrintString (Utilities|GetDisplayName (.HitActor (Collision|BreakHitResult _outhit))))))))
        (:then_1
          (Utilities|FlowControl|Delay 0.2)
          (goto _label Reset))))))

(event EventTake
  (params (Pawn :type Pawn%20Object%20Reference))
  (bind _self self)
  (if (not (Variables|Default|GetbIsUse))
    (bind _asjw_character (Utilities|Casting|CastToJW_Character Pawn))
    (Variables|Default|SetAs%20JW%20Character _asjw_character)
    (if (not (Utilities|IsValid (Variables|/Script/JoyWay_HEX512.JW_Character|GetWeaponFirst (Variables|Default|GetAs%20JW%20Character))))
      (Variables|/Script/JoyWay_HEX512.JW_Character|SetWeaponFirst (Variables|Default|GetAs%20JW%20Character) _self)
      (Transformation|AttachComponentToComponent self (Variables|/Script/JoyWay_HEX512.JW_Character|GetHandRightArm_Weapon (Variables|Default|GetAs%20JW%20Character)) "None" "SnapToTarget" "SnapToTarget" "SnapToTarget" true)
      (Actor|SetOwner (Variables|Default|GetAs%20JW%20Character) :!label _label)
      (Collision|SetCollisionResponsetoAllChannels (Variables|Default|GetWeaponMesh) "ECR_Ignore")
      (Variables|Default|SetbIsUse true)
      (Audio|Components|Audio|Play (Variables|Default|GetAudioRaise) 0.0)
      (elif (not (Utilities|IsValid (Variables|/Script/JoyWay_HEX512.JW_Character|GetWeaponSecond (Variables|Default|GetAs%20JW%20Character))))
        (Variables|/Script/JoyWay_HEX512.JW_Character|SetWeaponSecond (Variables|Default|GetAs%20JW%20Character) _self)
        (Transformation|AttachComponentToComponent self (Variables|/Script/JoyWay_HEX512.JW_Character|GetHandLeftArm_Weapon (Variables|Default|GetAs%20JW%20Character)) "None" "SnapToTarget" "SnapToTarget" "SnapToTarget" true)
        (goto _label)))))

(fn ConstructionScript)

(fn GetCurrentAmmo
  (return 0))